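; BP_Locked_Door is a hinged door for the dungeon generator that can start locked and opens with a matching key.
; A BP_DoorKey carrying the desired tag entering the box triggers Unlock and is optionally consumed.
; Unlock slides the latch on a timeline, then destroys it and swings the door open.
; Once unlocked, non-key overlaps play the hinge timeline and any end overlap reverses it.
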(event OnComponentBeginOverlap(Box)
  (params (OverlappedComponent :type Primitive%20Component%20Object%20Reference) (OtherActor :type Actor%20Object%20Reference) (OtherComp :type Primitive%20Component%20Object%20Reference) (OtherBodyIndex :type Integer) (bFromSweep :type Boolean) (SweepResult :type Hit%20Result%20Structure%20%28by%20ref%29))
  (bind _asbp_door_key (Utilities|Casting|CastToBP_DoorKey OtherActor)
    (:then
      (if (Actor|ActorHasTag OtherActor (Variables|Default|GetDesiredKeyTag))
        (CallFunction|Unlock)
        (if (Variables|Default|GetConsumeKey?)
          (Actor|DestroyActor _asbp_door_key))))
    (:CastFailed
      (if (not (Variables|Default|GetStartLocked?))
        (bind _newtrack_0 (Timeline|Door%20Open/Close Play)
          (:Update
            (Transformation|SetRelativeRotation (Variables|Default|GetHinge) (Math|Rotator|MakeRotator 0.0 0.0 _newtrack_0) false false)))))))

(event OnComponentEndOverlap(Box)
  (params (OverlappedComponent :type Primitive%20Component%20Object%20Reference) (OtherActor :type Actor%20Object%20Reference) (OtherComp :type Primitive%20Component%20Object%20Reference) (OtherBodyIndex :type Integer))
  (if (not (Variables|Default|GetStartLocked?))
    (bind _newtrack_0 (Timeline|Door%20Open/Close Reverse)
      (:Update
        (Transformation|SetRelativeRotation (Variables|Default|GetHinge) (Math|Rotator|MakeRotator 0.0 0.0 _newtrack_0) false false)))))

(event Custom|Unlock
  (Utilities|IsValid (Variables|Default|GetLatch)
    (:Is%20Valid
      (bind _unlatch (Timeline|Timeline Play)
        (:Update
          (Transformation|SetRelativeLocation (Variables|Default|GetLatch) (Math|Vector|MakeVector 0.0 _unlatch 0.0) false false))
        (:Finished
          (Variables|Default|SetStartLocked? false)
          (Components|DestroyComponent (Variables|Default|GetLatch))
          (bind _newtrack_0 (Timeline|Door%20Open/Close Play)
            (:Update
              (Transformation|SetRelativeRotation (Variables|Default|GetHinge) (Math|Rotator|MakeRotator 0.0 0.0 _newtrack_0) false false))))))))

(fn ConstructionScript
  (Rendering|Material|SetMaterial (Variables|Default|GetLatch) 0 (Variables|Default|GetMaterial)))