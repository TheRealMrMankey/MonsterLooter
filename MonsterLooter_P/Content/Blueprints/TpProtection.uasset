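; TpProtection is an overlap trigger that freezes player control while an actor is inside it, apparently to cover level loading around a teleport.
; Begin overlap prints a loading message and ignores player 0's look and move input, with no check on which actor entered.
; End overlap restores input, hides "Portal"-tagged actors and, nested in that loop, disables collision on the first "Box"-tagged component of each "PortalBP"-tagged actor.
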(event OnComponentBeginOverlap(Overlap)
  (params (OverlappedComponent :type Primitive%20Component%20Object%20Reference) (OtherActor :type Actor%20Object%20Reference) (OtherComp :type Primitive%20Component%20Object%20Reference) (OtherBodyIndex :type Integer) (bFromSweep :type Boolean) (SweepResult :type Hit%20Result%20Structure%20%28by%20ref%29))
  (bind _returnvalue (Game|GetPlayerController 0))
  (Development|PrintString "Loading Level")
  (Input|SetIgnoreLookInput _returnvalue true)
  (Input|SetIgnoreMoveInput _returnvalue true))

(event OnComponentEndOverlap(Overlap)
  (params (OverlappedComponent :type Primitive%20Component%20Object%20Reference) (OtherActor :type Actor%20Object%20Reference) (OtherComp :type Primitive%20Component%20Object%20Reference) (OtherBodyIndex :type Integer))
  (bind _returnvalue (Game|GetPlayerController 0))
  (Development|PrintString "Loaded")
  (Input|SetIgnoreLookInput _returnvalue false)
  (Input|SetIgnoreMoveInput _returnvalue false)
  (bind _outactors (Actor|GetAllActorswithTag "Portal"))
  (for _array_element _outactors
    (Rendering|SetActorHiddenInGame _array_element true)
    (bind _outactors_2 (Actor|GetAllActorswithTag "PortalBP"))
    (for _array_element_2 _outactors_2
      (bind _asprimitive_component (Utilities|Casting|CastToPrimitiveComponent (Utilities|Array|Get(acopy) (Actor|GetComponentsbyTag _array_element_2 "/Script/Engine.ActorComponent" "Box"))))
      (Collision|SetCollisionEnabled _asprimitive_component "NoCollision"))))

(fn ConstructionScript)