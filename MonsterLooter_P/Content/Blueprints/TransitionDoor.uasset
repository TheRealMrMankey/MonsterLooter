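; TransitionDoor is a door Blueprint that teleports a player between the outside world and a dungeon interior.
; Its Transition event plays a sound, then uses the InDungeon flag to move the player slightly above either the ExitTP or EntryTP location.
; It also finds the SunSky actor and shows its SkyLight outside or hides it inside, printing a debug string for each side.
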(event Custom|Transition
  (params (Player :type Rogue%20Object%20Reference) (InDungeon :type Boolean))
  (bind _entrytp (Variables|Default|GetEntryTP))
  (bind _exittp (Variables|Default|GetExitTP))
  (bind _returnvalue (Transformation|GetActorLocation _entrytp))
  (bind _returnvalue_2 (Transformation|GetActorLocation _exittp))
  (Audio|PlaySound2D "/Game/Audio/Misc/TransitionDoor.TransitionDoor" 1.0 1.0 0.0 0 0)
  (if InDungeon
    (Transformation|SetActorLocation Player (Math|Vector|MakeVector (.x _returnvalue_2) (.y _returnvalue_2) (+ (.z _returnvalue_2) 5e+01)) false true)
    (Development|PrintString "Im Outside")
    (bind _returnvalue_3 (Actor|GetActorOfClass "/SunPosition/SunSky.SunSky_C"))
    (Rendering|SetVisibility (Variables|/SunPosition/SunSky.SunSky_C|GetSkyLight _returnvalue_3) true false)
    (else
      (Transformation|SetActorLocation Player (Math|Vector|MakeVector (.x _returnvalue) (.y _returnvalue) (+ (.z _returnvalue) 1.2e+02)) false true)
      (Development|PrintString "Im Inside")
      (bind _returnvalue_4 (Actor|GetActorOfClass "/SunPosition/SunSky.SunSky_C"))
      (Rendering|SetVisibility (Variables|/SunPosition/SunSky.SunSky_C|GetSkyLight _returnvalue_4) false false))))

(fn ConstructionScript)