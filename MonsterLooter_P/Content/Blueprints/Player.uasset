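; Player controller Blueprint that routes jump, movement and look input to the player character.
; Movement follows control yaw, while look input adds yaw or pitch and calls UpdateHeadRot.
; UpdateHeadRot writes the control-to-character rotation offset into CharAnimBP's HeadRot and prints it for debugging.
; Beyond 90 degrees either side it updates a desired yaw, and it calls SetActorRotation on itself with an interpolated rotation.
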(event EventBeginPlay
  (Variables|Default|SetPlayerChar (Game|GetPlayerCharacter 0)))

(event Input|ActionEvents|InputActionJump
  (params (Key :type Key%20Structure :default "None"))
  (:Pressed
    (Character|Jump (Variables|Default|GetPlayerChar))))

(event Input|AxisEvents|InputAxisMoveForward
  (params (AxisValue :type Float%20%28single-precision%29))
  (Pawn|Input|AddMovementInput (Variables|Default|GetPlayerChar) (Math|Vector|GetForwardVector (Math|Rotator|MakeRotator 0.0 0.0 (.Yaw (Math|Rotator|BreakRotator (Pawn|GetControlRotation :!class /Script/Engine.Controller))))) AxisValue false))

(event Input|AxisEvents|InputAxisMoveRight
  (params (AxisValue :type Float%20%28single-precision%29))
  (Pawn|Input|AddMovementInput (Variables|Default|GetPlayerChar) (Math|Vector|GetRightVector (Math|Rotator|MakeRotator 0.0 0.0 (.Yaw (Math|Rotator|BreakRotator (Pawn|GetControlRotation :!class /Script/Engine.Controller))))) AxisValue false))

(event Input|AxisEvents|InputAxisTurn
  (params (AxisValue :type Float%20%28single-precision%29))
  (Class|PlayerController|AddYawInput AxisValue)
  (CallFunction|UpdateHeadRot))

(event Input|AxisEvents|InputAxisLookUp
  (params (AxisValue :type Float%20%28single-precision%29))
  (Class|PlayerController|AddPitchInput AxisValue)
  (CallFunction|UpdateHeadRot))

(fn ConstructionScript)

(fn UpdateHeadRot
  (bind _returnvalue (Pawn|GetControlRotation :!class /Script/Engine.Controller))
  (bind _playerchar (Variables|Default|GetPlayerChar))
  (bind _returnvalue_2 (Transformation|GetActorRotation _playerchar))
  (bind _returnvalue_3 (- (.yaw _returnvalue) (.yaw _returnvalue_2)))
  (bind _returnvalue_4 (Math|Float|ClampAngle _returnvalue_3 -179.0 -1.8e+02))
  (bind _aschar_anim_bp (Utilities|Casting|CastToCharAnimBP (Components|SkeletalMesh|GetAnimInstance (Variables|/Script/Engine.Character|GetMesh (Variables|Default|GetPlayerChar)))))
  (bind _output_get (Variables|/Game/Animation/CharAnimBP.CharAnimBP_C|SetHeadRot _aschar_anim_bp (Math|Rotator|MakeRotator (- 0.0 (.pitch _returnvalue)) 0.0 _returnvalue_3)))
  (Development|PrintString (Utilities|String|ToString(Rotator) _output_get))
  (if (> _returnvalue_4 9e+01)
    (Variables|Default|SetYawOffset 9e+01)
    (Variables|Default|SetDesiredYaw (+ (.yaw (Transformation|GetActorRotation (Variables|Default|GetPlayerChar))) (Variables|Default|GetYawOffset)) :!label _label)
    (elif (< _returnvalue_4 -9e+01)
      (Variables|Default|SetYawOffset -9e+01)
      (goto _label)
      (else
        _)))
  (Transformation|SetActorRotation (Math|Interpolation|RInterpTo (Transformation|GetActorRotation (Variables|Default|GetPlayerChar)) (Math|Rotator|MakeRotator 0.0 0.0 (Variables|Default|GetDesiredYaw)) (Utilities|Time|GetWorldDeltaSeconds) 5.0)))