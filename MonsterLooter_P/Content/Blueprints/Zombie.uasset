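; Zombie enemy that chases the Rogue player and kills it on contact, making it drop its items.
; PawnSensing sight or hearing starts the chase by raising walk speed and setting the HasHeardPlayer blackboard key for the AI.
; Tick ends the chase once the Rogue is beyond sight radius plus a margin, as does a kill.
; The capsule ignores killed Rogues and overlapped Doors when moving, letting it pass through them.
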(event OnHearNoise(PawnSensing)
  (params (Instigator :type Pawn%20Object%20Reference) (Location :type Vector%20%28by%20ref%29 :default "0, 0, 0") (Volume :type Float%20%28single-precision%29))
  ;[1 1 1] Chase Player
  (CallFunction|ChasePlayer Instigator))

(event OnSeePawn(PawnSensing)
  (params (Pawn :type Pawn%20Object%20Reference))
  ;[1 1 1] Chase Player
  (CallFunction|ChasePlayer Pawn))

(event OnComponentHit(CapsuleComponent)
  (params (HitComponent :type Primitive%20Component%20Object%20Reference) (OtherActor :type Actor%20Object%20Reference) (OtherComp :type Primitive%20Component%20Object%20Reference) (NormalImpulse :type Vector :default "0, 0, 0") (Hit :type Hit%20Result%20Structure%20%28by%20ref%29))
  ;[1 1 1] Kill player on hit
  (bind _asrogue (Utilities|Casting|CastToRogue OtherActor))
  (Default|Die _asrogue)
  (Default|DropItems _asrogue)
  (CallFunction|StopChasing)
  (Collision|IgnoreActorwhenMoving (Variables|Collision|GetCapsuleComponent) _asrogue true))

(event OnComponentBeginOverlap(CapsuleComponent)
  (params (OverlappedComponent :type Primitive%20Component%20Object%20Reference) (OtherActor :type Actor%20Object%20Reference) (OtherComp :type Primitive%20Component%20Object%20Reference) (OtherBodyIndex :type Integer) (bFromSweep :type Boolean) (SweepResult :type Hit%20Result%20Structure%20%28by%20ref%29))
  (bind _asdoor (Utilities|Casting|CastToDoor OtherActor))
  (Collision|IgnoreActorwhenMoving (Variables|Collision|GetCapsuleComponent) _asdoor true))

(event Custom|Chase%20Player
  (params (Target :type Actor%20Object%20Reference))
  ;[1 1 1] Chase Player
  (bind _asrogue (Utilities|Casting|CastToRogue Target))
  (Variables|Default|SetAs%20Rogue _asrogue)
  (Variables|/Script/Engine.CharacterMovementComponent|SetMaxWalkSpeed (Variables|Character|GetCharacterMovement) (Variables|Default|GetMonsterChaseSpeed))
  (AI|Components|Blackboard|SetValueasBool (AI|GetBlackboard (AI|GetAIController self)) (Utilities|Name|MakeLiteralName "HasHeardPlayer") true)
  (Variables|Default|SetHasTarget true))

(event Custom|Stop%20Chasing
  ;[1 1 1] Stop Chasing
  (AI|Components|Blackboard|SetValueasBool (AI|GetBlackboard (AI|GetAIController self)) (Utilities|Name|MakeLiteralName "HasHeardPlayer") false)
  (Variables|Default|SetHasTarget false)
  (Variables|/Script/Engine.CharacterMovementComponent|SetMaxWalkSpeed (Variables|Character|GetCharacterMovement) (Variables|Default|GetMonsterWalkSpeed)))

(event EventTick
  (params (DeltaSeconds :type Float%20%28single-precision%29))
  ;[1 1 1] Check if player is still in hearing range
  (if (Variables|Default|GetHasTarget)
    (if (> (Transformation|GetDistanceTo (Variables|Default|GetAs%20Rogue)) (+ (Variables|/Script/AIModule.PawnSensingComponent|GetSightRadius (Variables|Default|GetPawnSensing)) 3e+02))
      (CallFunction|StopChasing)
      (Variables|Default|SetHasTarget false)
      (Variables|/Script/Engine.CharacterMovementComponent|SetMaxWalkSpeed (Variables|Character|GetCharacterMovement) (Variables|Default|GetMonsterWalkSpeed)))))

(fn ConstructionScript)