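; Portal actor that teleports every Rogue between the Tavern and Desert destination portals when overlapped.
; Overlap passes through a server RPC to RPC_Overlap, which reads GlobalTracker's selected level and places Rogues at the destination's Plane, spaced along X.
; It then updates the current level, flips the selection for the next trip, and calls SedSeed on Desert arrivals.
; Box collision starts disabled at BeginPlay.
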(event Custom|RPC_Server_Overlap
  (CallFunction|RPCOverlap))

(event Custom|RPC_Overlap
  (bind _returnvalue (Actor|GetActorOfClass "/Game/Blueprints/GlobalTracker.GlobalTracker_C"))
  (Variables|Default|SetAs%20GT _returnvalue)
  (bind _outactors (Actor|GetAllActorsOfClass "/Game/Blueprints/Rogue.Rogue_C"))
  (for (_array_element _array_index) _outactors
    (if (Utilities|Enum|Equal(Enum) (Variables|/Game/Blueprints/GlobalTracker.GlobalTracker_C|GetSelectedLevel (Variables|Default|GetAs%20GT)) "Tavern")
      (bind _asportal (Utilities|Casting|CastToPortal (Variables|Default|GetTavernDestination)))
      (Transformation|SetActorLocation _array_element (Math|Vector|MakeVector (+ (* _array_index 50) (.x (Transformation|GetWorldLocation (Variables|Portal_C|GetPlane _asportal)))) (.y (Transformation|GetWorldLocation (Variables|Portal_C|GetPlane _asportal))) (.z (Transformation|GetWorldLocation (Variables|Portal_C|GetPlane _asportal)))) false true)
      (Variables|/Game/Blueprints/GlobalTracker.GlobalTracker_C|SetCurrentLevel (Variables|Default|GetAs%20GT) "Tavern")
      (elif (Utilities|Enum|Equal(Enum) (Variables|/Game/Blueprints/GlobalTracker.GlobalTracker_C|GetSelectedLevel (Variables|Default|GetAs%20GT)) "Desert")
        (bind _asportal_2 (Utilities|Casting|CastToPortal (Variables|Default|GetDesertDestination)))
        (Transformation|SetActorLocation _array_element (Math|Vector|MakeVector (+ (.x (Transformation|GetWorldLocation (Variables|Portal_C|GetPlane _asportal_2))) (* _array_index 5e+01)) (.y (Transformation|GetWorldLocation (Variables|Portal_C|GetPlane _asportal_2))) (.z (Transformation|GetWorldLocation (Variables|Portal_C|GetPlane _asportal_2)))) false true)
        (Variables|/Game/Blueprints/GlobalTracker.GlobalTracker_C|SetCurrentLevel (Variables|Default|GetAs%20GT) "Desert")
        (Default|SedSeed (Variables|Default|GetAs%20GT)))))
  (if (Utilities|Enum|Equal(Enum) (Variables|/Game/Blueprints/GlobalTracker.GlobalTracker_C|GetCurrentLevel (Variables|Default|GetAs%20GT)) "Tavern")
    (Variables|/Game/Blueprints/GlobalTracker.GlobalTracker_C|SetSelectedLevel (Variables|Default|GetAs%20GT) "Desert")
    (Variables|/Game/Blueprints/GlobalTracker.GlobalTracker_C|SetCurrentLevel (Variables|Default|GetAs%20GT) "Tavern")
    (elif (Utilities|Enum|Equal(Enum) (Variables|/Game/Blueprints/GlobalTracker.GlobalTracker_C|GetCurrentLevel (Variables|Default|GetAs%20GT)) "Desert")
      (Variables|/Game/Blueprints/GlobalTracker.GlobalTracker_C|SetSelectedLevel (Variables|Default|GetAs%20GT) "Tavern")
      (Variables|/Game/Blueprints/GlobalTracker.GlobalTracker_C|SetCurrentLevel (Variables|Default|GetAs%20GT) "Desert"))))

(event EventBeginPlay
  (Collision|SetCollisionEnabled (Variables|Default|GetBox) "NoCollision"))

(event Collision|EventActorBeginOverlap
  (params (OtherActor :type Actor%20Object%20Reference))
  (CallFunction|RPCServerOverlap))

(fn ConstructionScript)