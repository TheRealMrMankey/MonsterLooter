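; DungeonMusic switches between outside and dungeon audio, starting with the outside track at BeginPlay.
; Two events, StopDungeonAudio and StopOutsideAudio, each stop one track and start the other.
; A near-endless delayed loop, spaced by ScaryNoiseTime, checks the Rogue's InDungeon flag, restarting RandomNoises when it is false and stopping them when it is true.
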(event Custom|StopOutsideAudio
  (Audio|Components|Audio|Play (Variables|Default|GetDungeonAudio) 0.0)
  (Audio|Components|Audio|Stop (Variables|Default|GetOutsideAudio)))

(event Custom|StopDungeonAudio
  (Audio|Components|Audio|Stop (Variables|Default|GetDungeonAudio))
  (Audio|Components|Audio|Play (Variables|Default|GetOutsideAudio) 0.0))

(event EventBeginPlay
  (Audio|Components|Audio|Stop (Variables|Default|GetDungeonAudio))
  (Audio|Components|Audio|Play (Variables|Default|GetOutsideAudio) 0.0)
  (Utilities|ForLoopwithDelay 0 99999 (Variables|Default|GetScaryNoiseTime)
    (:Loop%20Body
      (bind _returnvalue (Actor|GetActorOfClass "/Game/Blueprints/Rogue.Rogue_C"))
      (if (Variables|/Game/Blueprints/Rogue.Rogue_C|GetInDungeon _returnvalue)
        (Audio|Components|Audio|Stop (Variables|Default|GetRandomNoises))
        (else
          (Audio|Components|Audio|Play (Variables|Default|GetRandomNoises) 0.0))))))

(fn ConstructionScript)